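; Placeable, upgradeable tower defense cannon that shoots zombies in range, shown collisionless with a flat material until placement is finalized.
; Sphere overlaps maintain a target queue, from which Tick picks the first zombie as target.
; A looping timer started on placement spawns homing projectiles and applies damage immediately on firing, not on impact.
; Upgrades spend GameManager money and reload stats from DTCannon, but leave the running timer's interval unchanged.
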(event `self.ReceiveBeginPlay`
  (if (`self.bIsPlaced`)
    (set `self.bIsPlaced` true)
    (`self.UpdateCannonStats`)
    (else
      (`PrimitiveComponent.SetCollisionEnabled` (`self.Cube`) "NoCollision")
      (`PrimitiveComponent.SetCollisionEnabled` (`self.Sphere`) "NoCollision")
      (`PrimitiveComponent.SetMaterial` (`self.Cube`) 0 "/Game/LevelPrototyping/Materials/M_FlatCol.M_FlatCol"))))

(event `TryToUpgrade`
  (bind _outactors (`GameplayStatics.GetAllActorsOfClass` "/Game/BP_Coin/BP_GameManager.BP_GameManager_C"))
  (bind _asbp_game_manager (cast `/Game/BP_Coin/BP_GameManager` (`|GetArrayItem` _outactors)))
  (`/Game/BP_Coin/BP_GameManager.SpendMoney` _asbp_game_manager (`self.UpgradeCost`))
  (if (`/Game/BP_Coin/BP_GameManager.WasSuccessful` _asbp_game_manager)
    (bind _output_get (set `self.UpgradeLevel` (+ (`self.UpgradeLevel`) 1)))
    (set `self.RowName` (select `int` _output_get :`0` "None" :`1` "1" :`2` "2" :`3` "3" :!type "Name"))
    (`self.UpdateCannonStats`)
    (else
      (`KismetSystemLibrary.PrintString` "Not ENough Money"))))

(event `FinalizePlacement`
  (set `self.bIsPlaced` true)
  (`PrimitiveComponent.SetMaterial` (`self.Cube`) 0 "/Game/Cannon/M_Cannon.M_Cannon")
  (`PrimitiveComponent.SetCollisionEnabled` (`self.Cube`) "QueryAndPhysics")
  (`PrimitiveComponent.SetCollisionEnabled` (`self.Sphere`) "QueryAndPhysics")
  (`self.UpdateCannonStats`)
  (`KismetSystemLibrary.K2_SetTimer` self "FireCannon" (`self.FireRate`) true))

(event `self.Sphere.OnComponentBeginOverlap`
  (params (OverlappedComponent :type "PrimitiveComponent Object Reference") (OtherActor :type "Actor Object Reference") (OtherComp :type "PrimitiveComponent Object Reference") (OtherBodyIndex :type Integer) (bFromSweep :type Boolean) (SweepResult :type "HitResult Structure (by ref)"))
  (bind _asbp_zombie (cast `/Game/Zombie/BP_Zombie` OtherActor))
  (`KismetArrayLibrary.Array_Add` (`self.TargetQueue`) _asbp_zombie))

(event `FireCannon`
  (bind _targetzombie (`self.TargetZombie`))
  (`/Engine/EditorBlueprintResources/StandardMacros.IsValid` _targetzombie
    (:`Is Valid`
      (if true
        (bind _returnvalue (`|SpawnActorFromClass` (`self.ProjectileClass`) (`SceneComponent.K2_GetComponentToWorld` (`self.Muzzle`)) "Undefined" "MultiplyWithRoot" null null))
        (set `ProjectileMovementComponent.HomingTargetComponent` (`Character.CapsuleComponent` (`self.TargetZombie`)) (`self.GetComponentByClass` _returnvalue "/Script/Engine.ProjectileMovementComponent"))
        (`GameplayStatics.ApplyDamage` (`self.TargetZombie`) (`self.Damage`) null self)
        (else
          (`/Engine/EditorBlueprintResources/StandardMacros.IsValid` (`|GetArrayItem` (`PrimitiveComponent.GetOverlappingActors` (`self.Sphere`) "/Game/Zombie/BP_Zombie.BP_Zombie_C"))
            (:`Is Valid`
              (if true
                (set `self.TargetZombie` _targetzombie)
                (else
                  (set `self.TargetZombie` null)
                  (`KismetSystemLibrary.K2_ClearTimer` null "FireCannon"))))))))))

(event `self.Sphere.OnComponentEndOverlap`
  (params (OverlappedComponent :type "PrimitiveComponent Object Reference") (OtherActor :type "Actor Object Reference") (OtherComp :type "PrimitiveComponent Object Reference") (OtherBodyIndex :type Integer))
  (bind _asbp_zombie (cast `/Game/Zombie/BP_Zombie` OtherActor))
  (`KismetArrayLibrary.Array_RemoveItem` (`self.TargetQueue`) _asbp_zombie))

(event `self.ReceiveTick`
  (params (DeltaSeconds :type "Float (single-precision)"))
  (if (> (`KismetArrayLibrary.Array_Length` (`self.TargetQueue`)) 0)
    (`/Engine/EditorBlueprintResources/StandardMacros.IsValid` (`|GetArrayItem` (`self.TargetQueue`))
      (:`Is Valid`
        (if true
          (if (`self.bCanFire`)
            (set `self.bCanFire` false)
            (set `self.TargetZombie` (`|GetArrayItem` (`self.TargetQueue`)))
            (`KismetSystemLibrary.Delay` (`self.FireRate`))
            (set `self.bCanFire` true))
          (else
            (`KismetArrayLibrary.Array_Remove` (`self.TargetQueue`))))))))

(fn `UpdateCannonStats`
  (bind _returnvalue (`|GetDataTableRow` (`self.DT_Cannon`) (`self.RowName`))
    (:`then`
      (bind (_damage _firerate _range _upgradecost _upgradelevel _fireball) (break `/Game/Cannon/ST_Cannon` _returnvalue))
      (set `self.Damage` _damage)
      (set `self.FireRate` _firerate)
      (`SphereComponent.SetSphereRadius` (`self.Sphere`) _range true)
      (set `self.UpgradeCost` _upgradecost)
      (set `self.UpgradeLevel` _upgradelevel)
      (set `self.ProjectileClass` _fireball))))

(fn `UserConstructionScript`)