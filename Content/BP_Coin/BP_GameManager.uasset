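; BP_GameManager tracks the player's money and shows it on screen through a Money_Widget created at BeginPlay.
; AddMoney increases PlayerMoney and pushes the new total to the widget.
; SpendMoney returns whether PlayerMoney covers a cost.
; Its deduction and widget update sit on a Sequence pin after the one that returns true, so the Return node precedes them.
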(event `self.ReceiveBeginPlay`
  (bind _returnvalue (`|CreateWidget` "/Game/BP_Coin/Money_Widget.Money_Widget_C"))
  (bind _output_get (set `self.Widget` _returnvalue))
  (`UserWidget.AddToViewport` _output_get 0))

(fn `AddMoney`
  (params (Amount :type Integer))
  (bind _returnvalue (+ (`self.PlayerMoney`) Amount))
  (bind _output_get (set `self.Money` _returnvalue))
  (`/Game/BP_Coin/Money_Widget.UpdateMoney` (`self.Widget`) _output_get)
  (set `self.PlayerMoney` _returnvalue))

(fn `SpendMoney`
  (params (Cost :type Integer :default 0))
  (returns (bWasSuccessful :type Boolean))
  (if (>= (`self.PlayerMoney`) Cost)
    (`|ExecutionSequence`
      (:`then_0`
        (return true))
      (:`then_1`
        (bind _output_get (set `self.Money` (`self.PlayerMoney`)))
        (bind _returnvalue (- _output_get Cost))
        (bind _output_get_2 (set `self.Money` _returnvalue))
        (`/Game/BP_Coin/Money_Widget.UpdateMoney` (`self.Widget`) _output_get_2)
        (set `self.PlayerMoney` _returnvalue)))
    (else
      (return false))))

(fn `UserConstructionScript`)